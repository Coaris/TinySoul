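; BP_Player is the player character Blueprint, handling movement, camera look and jumping.
; Enhanced Input actions drive camera-relative movement from control yaw, add yaw and inverted pitch to the controller, and trigger Jump.
; A SetLandState event sets IsLanding, which blocks movement input during the landing animation.
; BeginPlay caches the mesh's Anim Instance.
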(event Input|EnhancedActionEvents|EnhancedInputActionIA_Move
  (params (ActionValue :type Vector%202D%20Structure) (ElapsedSeconds :type Float%20%28double-precision%29) (TriggeredSeconds :type Float%20%28double-precision%29) (InputAction :type Input%20Action%20Object%20Reference :default "/Game/Jiale/Misc/Inputs/IA_Move.IA_Move"))
  (bind _returnvalue (Pawn|GetControlRotation :!class /Script/Engine.Pawn))
  ;[1 1 1] 控制角色移动/input action for character's movement
  (:Triggered
    (if (not (Variables|Default|GetIsLanding))
      ;;[1 1 1] W/S move forward or backward
      (Pawn|Input|AddMovementInput (Math|Vector|GetForwardVector (Math|Rotator|MakeRotator 0.0 0.0 (.yaw _returnvalue))) (.y ActionValue) false)
      ;;[1 1 1] A/D move left or right
      (Pawn|Input|AddMovementInput (Math|Vector|GetRightVector (Math|Rotator|MakeRotator 0.0 0.0 (.yaw _returnvalue))) (.x ActionValue) false))))

(event Input|EnhancedActionEvents|EnhancedInputActionIA_CameraControl
  (params (ActionValue :type Vector%202D%20Structure) (ElapsedSeconds :type Float%20%28double-precision%29) (TriggeredSeconds :type Float%20%28double-precision%29) (InputAction :type Input%20Action%20Object%20Reference :default "/Game/Jiale/Misc/Inputs/IA_CameraControl.IA_CameraControl"))
  ;[1 1 1] 相机控制/Camera rotation control
  (:Triggered
    (Pawn|Input|AddControllerYawInput (.x ActionValue))
    (Pawn|Input|AddControllerPitchInput (* (.y ActionValue) -1.0))))

(event Input|EnhancedActionEvents|EnhancedInputActionIA_Jump
  (params (ActionValue :type Boolean) (ElapsedSeconds :type Float%20%28double-precision%29) (TriggeredSeconds :type Float%20%28double-precision%29) (InputAction :type Input%20Action%20Object%20Reference :default "/Game/Jiale/Misc/Inputs/IA_Jump.IA_Jump"))
  (:Started
    (Character|Jump)))

(event EventSetLandState
  (params (LandingState :type Boolean))
  ;[1 1 1] 当处于着陆动画时，玩家不能移动/ Player can't move when character is landing
  (Variables|Default|SetIsLanding LandingState))

(event EventBeginPlay
  ;[1 1 1] Get ABP_PLayer's Anim instance
  (Variables|Default|SetAnimInstance (Components|SkeletalMesh|GetAnimInstance (Variables|Character|GetMesh))))

(fn ConstructionScript)